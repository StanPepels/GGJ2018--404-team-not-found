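; Duck actor that is steered by the tiles it overlaps and triggers the lose screen when destroyed.
; Overlaps turn it after a delay by the tile's Action, or zero MoveSpeed against obstacles and other ducks until contact ends.
; Flesh-eating plants, or leaving hardcoded screen bounds checked on Tick, flag it via AutoDestroyWhenFinished; Destroyed pauses the game and passes duck and culprit names to LoseScreen.
; MovedTile toggles every mole's state.
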(event Custom|MovedTile
  (bind _outactors (Actor|GetAllActorsOfClass "/Game/Blueprints/Obstacles/bp_Mole.bp_Mole_C"))
  (for _array_element _outactors
    (Default|ToggleState _array_element)))

(event EventTick
  (params (DeltaSeconds :type Float%20%28single-precision%29))
  (bind _returnvalue (Transformation|GetActorLocation))
  (bind _returnvalue_2 (Game|GetPlayerController 0))
  (bind _screenposition (Class|GameplayStatics|ProjectWorldtoScreen _returnvalue_2 _returnvalue false))
  (Utilities|FlowControl|Sequence
    (:then_0
      (Utilities|FlowControl|Delay 2.0)
      (if (Math|Boolean|ORBoolean (<= (.x _screenposition) -5e+01) (<= (.y _screenposition) -5e+01) (>= (.y _screenposition) 1.1e+03) (>= (.x _screenposition) 1.92e+03))
        (Variables|Default|SetbAutoDestroyWhenFinished true)))
    (:then_1
      (if (Variables|Default|GetStopped)
        _))))

(event Collision|EventActorBeginOverlap
  (params (OtherActor :type Actor%20Object%20Reference))
  (Utilities|FlowControl|Sequence
    (:then_0
      (bind _asbp_test_tile (Utilities|Casting|CastTobp_TestTile OtherActor))
      (Utilities|FlowControl|Delay 2.0)
      (if (== (Variables|Default|GetMoveSpeed) 0.0)
        (Variables|Default|SetMoveSpeed 5.0))
      (switch Utilities|FlowControl|Switch|SwitchonAction (Variables|/Game/Blueprints/Testing/bp_TestTile.bp_TestTile_C|GetAction _asbp_test_tile)
        (:NewEnumerator0
          (Transformation|SetActorRotation (Math|Rotator|MakeRotator 0.0 0.0 -9e+01)))
        (:NewEnumerator1
          (Transformation|SetActorRotation (Math|Rotator|MakeRotator 0.0 0.0 9e+01)))
        (:NewEnumerator2
          (Transformation|SetActorRotation (Math|Rotator|MakeRotator 0.0 0.0 1.8e+02)))
        (:NewEnumerator3
          (Transformation|SetActorRotation (Math|Rotator|MakeRotator 0.0 0.0 0.0)))))
    (:then_1
      (bind _asbp_flesh_eating_plant (Utilities|Casting|CastTobp_FleshEatingPlant OtherActor))
      (Variables|Default|SetObjectName (Variables|/Game/Blueprints/Obstacles/bp_FleshEatingPlant.bp_FleshEatingPlant_C|GetName _asbp_flesh_eating_plant))
      (Development|PrintString "The plant has devoured you")
      (Variables|Default|SetbAutoDestroyWhenFinished true))
    (:then_2
      (bind _asbp_static_obstacle (Utilities|Casting|CastTobp_StaticObstacle OtherActor))
      (Variables|Default|SetMoveSpeed 0.0)
      (Variables|Default|SetObjectName (Variables|/Game/Blueprints/Obstacles/bp_StaticObstacle.bp_StaticObstacle_C|GetName _asbp_static_obstacle)))
    (:then_3
      (Utilities|Casting|CastTobp_Duck OtherActor)
      (Variables|Default|SetMoveSpeed 0.0))))

(event Collision|EventActorEndOverlap
  (params (OtherActor :type Actor%20Object%20Reference))
  (Utilities|FlowControl|Sequence
    (:then_0
      (Utilities|Casting|CastTobp_StaticObstacle OtherActor)
      (Variables|Default|SetMoveSpeed 5.0))
    (:then_1
      (Utilities|Casting|CastTobp_Duck OtherActor)
      (Variables|Default|SetMoveSpeed 5.0))))

(event EventDestroyed
  (bind _returnvalue (UserInterface|CreateWidget "/Game/UI/LoseScreen.LoseScreen_C" (Game|GetPlayerController 0)))
  (Variables|/Game/UI/LoseScreen.LoseScreen_C|SetDuckName _returnvalue (Variables|Default|GetName))
  (Variables|/Game/UI/LoseScreen.LoseScreen_C|SetObjectName _returnvalue (Variables|Default|GetObjectName))
  (UserInterface|Viewport|AddtoViewport _returnvalue 0)
  (Game|SetGamePaused true))

(fn ConstructionScript)