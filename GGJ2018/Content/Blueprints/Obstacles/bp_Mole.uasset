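; Mole obstacle that switches between raised and lowered states, moving itself vertically on each ToggleState call.
; When it rises, it queries its Cube component for overlapping Bp_Duck actors.
; Each duck found is shifted back one tile length along its local negative Y axis and has its move speed set to zero.
; The toggle has no trigger or timer in this Blueprint.
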(event Custom|ToggleState
  (bind _cube (Variables|Default|GetCube))
  (if (Utilities|Enum|Equal(Enum) (Variables|Default|GetState) "NewEnumerator0")
    (Variables|Default|SetState "NewEnumerator1")
    (Transformation|AddActorLocalOffset "0.0,0.0,-300.000000" false false)
    (else
      (Variables|Default|SetState "NewEnumerator0")
      (Transformation|AddActorLocalOffset "0.0,0.0,300.000000" false false)
      (bind _outactors (Collision|ComponentOverlapActors _cube (Transformation|GetWorldTransform _cube) (Utilities|Array|MakeArray "ObjectTypeQuery2") "/Game/Blueprints/AI/bp_Duck.bp_Duck_C"))
      (for _array_element _outactors
        (bind _asbp_duck (Utilities|Casting|CastTobp_Duck _array_element))
        (Transformation|AddActorLocalOffset _asbp_duck (Math|Vector|MakeVector 0.0 (* (Variables|/Game/Blueprints/AI/bp_Duck.bp_Duck_C|GetTileLenght _asbp_duck) -1.0) 0.0) false false)
        (Variables|/Game/Blueprints/AI/bp_Duck.bp_Duck_C|SetMoveSpeed _asbp_duck 0.0)))))

(fn ConstructionScript)