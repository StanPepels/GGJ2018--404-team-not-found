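; Pickup actor that adds one use to the matching inventory item when a bp_Duck overlaps its Box.
; On overlap it gets the InventoryBar through bp_GameMode and loops over its NormalInventorySlot children.
; The first slot whose ItemToSpawn matches the pickup's Type has its NumUses incremented.
; It prints the slot count as debug output and does not destroy itself in this graph.
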(event OnComponentHit(Box)
  (params (HitComponent :type Primitive%20Component%20Object%20Reference) (OtherActor :type Actor%20Object%20Reference) (OtherComp :type Primitive%20Component%20Object%20Reference) (NormalImpulse :type Vector :default "0, 0, 0") (Hit :type Hit%20Result%20Structure%20%28by%20ref%29)))

(event OnComponentBeginOverlap(Box)
  (params (OverlappedComponent :type Primitive%20Component%20Object%20Reference) (OtherActor :type Actor%20Object%20Reference) (OtherComp :type Primitive%20Component%20Object%20Reference) (OtherBodyIndex :type Integer) (bFromSweep :type Boolean) (SweepResult :type Hit%20Result%20Structure%20%28by%20ref%29))
  (Utilities|Casting|CastTobp_Duck OtherActor)
  (bind _asbp_game_mode (Utilities|Casting|CastTobp_GameMode (Game|GetGameMode)))
  (Development|PrintString (Utilities|String|ToString(Integer) (Class|PanelWidget|GetChildrenCount (Variables|/Game/UI/InventoryBar.InventoryBar_C|GetInventory_bar (Variables|/Game/Blueprints/bp_GameMode.bp_GameMode_C|Getinventory _asbp_game_mode)))))
  (bind _result (Math|Integer|DecrementInt (Class|PanelWidget|GetChildrenCount (Variables|/Game/UI/InventoryBar.InventoryBar_C|GetInventory_bar (Variables|/Game/Blueprints/bp_GameMode.bp_GameMode_C|Getinventory _asbp_game_mode))))
    (:%20%20
      (bind _index (Utilities|FlowControl|ForLoopwithBreak 0 _result :!label _label)
        (:LoopBody
          (bind _asnormal_inventory_slot (Utilities|Casting|CastToNormalInventorySlot (Class|PanelWidget|GetChildat (Variables|/Game/UI/InventoryBar.InventoryBar_C|GetInventory_bar (Variables|/Game/Blueprints/bp_GameMode.bp_GameMode_C|Getinventory _asbp_game_mode)) _index)))
          (if (Utilities|Enum|Equal(Enum) (Variables|/Game/UI/NormalInventorySlot.NormalInventorySlot_C|GetItemToSpawn _asnormal_inventory_slot) (Variables|Default|Gettype))
            (bind _result_2 (Math|Integer|IncrementInt (Variables|/Game/UI/NormalInventorySlot.NormalInventorySlot_C|Getnum_uses _asnormal_inventory_slot))
              (:%20%20
                (Variables|/Game/UI/NormalInventorySlot.NormalInventorySlot_C|Setnum_uses _asnormal_inventory_slot _result_2)
                (goto _label Break)))))))))

(event EventBeginPlay)

(event Collision|EventActorBeginOverlap
  (params (OtherActor :type Actor%20Object%20Reference)))

(event EventTick
  (params (DeltaSeconds :type Float%20%28single-precision%29)))

(fn ConstructionScript)