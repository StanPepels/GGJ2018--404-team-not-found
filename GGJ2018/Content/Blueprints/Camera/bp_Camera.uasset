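; Side-scrolling camera pawn that player controller 0 possesses on BeginPlay, falling back to the first BP_Grid in the level if none is set.
; Space toggles a Gate fed by Tick, which moves the Arrow along its local Y by ScrollSpeed scaled by delta time.
; While scrolling, it passes the Camera's world location to the grid's UpdateGrid each frame.
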(event EventBeginPlay
  (Pawn|Possess (Game|GetPlayerController 0) self)
  (Utilities|IsValid (Variables|Default|GetGrid)
    (:Is%20Not%20Valid
      (bind _outactors (Actor|GetAllActorsOfClass "/Game/Blueprints/BP_Grid.BP_Grid_C"))
      (Variables|Default|SetGrid (Utilities|Array|Get(acopy) _outactors)))))

(event EventTick
  (params (DeltaSeconds :type Float%20%28single-precision%29))
  (bind _grid (Variables|Default|GetGrid))
  ;[1 1 1] Side scrolling
  (Utilities|FlowControl|Gate true
    (:Exit
      (Transformation|AddLocalOffset (Variables|Default|GetArrow) (Math|Vector|MakeVector 0.0 (* (Variables|Default|GetScrollSpeed) DeltaSeconds) 0.0) false false)
      (Utilities|IsValid _grid
        (:Is%20Valid
          (Default|UpdateGrid _grid (Transformation|GetWorldLocation (Variables|Default|GetCamera))))))))

(event Input|KeyboardEvents|SpaceBar
  (params (Key :type Key%20Structure))
  (bind _grid (Variables|Default|GetGrid))
  ;[1 1 1] Side scrolling
  (:Pressed
    (Utilities|FlowControl|Gate true) ; enters at Toggle
  ))

(fn ConstructionScript
  (bind _springarm (Variables|Default|GetSpringArm))
  (bind _returnvalue (Transformation|GetWorldLocation _springarm))
  (Transformation|SetWorldLocation _springarm (Math|Vector|MakeVector (.x _returnvalue) (.y _returnvalue) 0.0) false false))