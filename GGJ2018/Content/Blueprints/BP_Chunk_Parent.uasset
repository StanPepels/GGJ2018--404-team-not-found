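; BP_Chunk_Parent is a base level chunk that stores a square grid of tile types such as walkable, obstacle and death zone.
; The construction script sizes the layout array and draws temporary debug boxes, blue for obstacles and red for death zones.
; GetTile maps a position to its tile type and center through GetTileXY.
; IsCompatible requires at least one aligned walkable pair between this chunk's last row and another's first.
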(event EventBeginPlay)

(event Collision|EventActorBeginOverlap
  (params (OtherActor :type Actor%20Object%20Reference)))

(event EventTick
  (params (DeltaSeconds :type Float%20%28single-precision%29)))

(fn ConstructionScript
  (bind _tilesinchunk (Variables|Default|GetTilesInChunk))
  (bind _tilesize (Variables|Default|GetTileSize))
  (bind _tilesize_2 (Variables|Default|GetTileSize))
  (bind _returnvalue (- _tilesinchunk 1))
  (bind _returnvalue_2 (* _tilesize 0.5))
  (bind _returnvalue_3 (Math|Conversions|ToVector(Float) _returnvalue_2))
  (Variables|Default|SetChunkSize (* (Variables|Default|GetTilesInChunk) (Variables|Default|GetTileSize)))
  (Utilities|Array|Resize (Variables|Default|GetTileLayout) (* (Variables|Default|GetTilesInChunk) (Variables|Default|GetTilesInChunk)))
  (for _index (range 0 _returnvalue)
    (for _index_2 (range 0 _returnvalue)
      (bind _tile (CallFunction|GetTileXY _index _index_2))
      (switch Utilities|FlowControl|Switch|SwitchonTileType _tile
        (:NewEnumerator1
          (Rendering|Debug|DrawDebugBox (Math|Vector|MakeVector (.x (- (* (+ (Math|Vector|MakeVector (Math|Conversions|ToFloat(Integer) _index) (Math|Conversions|ToFloat(Integer) _index_2) 0.0) 0.5) _tilesize) (* (Variables|Default|GetChunkSize) 0.5))) (.y (- (* (+ (Math|Vector|MakeVector (Math|Conversions|ToFloat(Integer) _index) (Math|Conversions|ToFloat(Integer) _index_2) 0.0) 0.5) _tilesize) (* (Variables|Default|GetChunkSize) 0.5))) 0.0) (Math|Vector|MakeVector (.x _returnvalue_3) (.y _returnvalue_3) _tilesize_2) "(R=0.000000,G=0.000000,B=1.000000,A=1.000000)" "0, 0, 0" 2.0 1e+01))
        (:NewEnumerator2
          (Rendering|Debug|DrawDebugBox (Math|Vector|MakeVector (.x (- (* (+ (Math|Vector|MakeVector (Math|Conversions|ToFloat(Integer) _index) (Math|Conversions|ToFloat(Integer) _index_2) 0.0) 0.5) _tilesize) (* (Variables|Default|GetChunkSize) 0.5))) (.y (- (* (+ (Math|Vector|MakeVector (Math|Conversions|ToFloat(Integer) _index) (Math|Conversions|ToFloat(Integer) _index_2) 0.0) 0.5) _tilesize) (* (Variables|Default|GetChunkSize) 0.5))) 0.0) (Math|Vector|MakeVector (.x _returnvalue_3) (.y _returnvalue_3) _tilesize_2) "(R=1.000000,G=0.000000,B=0.000000,A=1.000000)" "0, 0, 0" 2.0 1e+01))))))

(fn GetTile
  (params (Position :type Vector))
  (bind _defaultsceneroot (Variables|Default|GetDefaultSceneRoot))
  (bind _tilesize (Variables|Default|GetTileSize))
  (bind _chunksize (Variables|Default|GetChunkSize))
  (bind _tilesize_2 (Variables|Default|GetTileSize))
  (bind _returnvalue (/ Position _tilesize))
  (bind _returnvalue_2 (Transformation|GetWorldLocation _defaultsceneroot))
  (bind _returnvalue_3 (* _chunksize 0.5))
  (bind _returnvalue_4 (Class|KismetMathLibrary|FTruncVector _returnvalue))
  (bind _returnvalue_5 (- _returnvalue_2 _returnvalue_3))
  (bind _returnvalue_6 (Math|Conversions|ToFloat(Integer) (.x _returnvalue_4)))
  (bind _returnvalue_7 (Math|Conversions|ToFloat(Integer) (.y _returnvalue_4)))
  (bind _returnvalue_8 (+ _returnvalue_6 0.5))
  (bind _returnvalue_9 (+ _returnvalue_7 0.5))
  (bind _returnvalue_10 (Math|Vector|MakeVector _returnvalue_8 _returnvalue_9 0.0))
  (bind _returnvalue_11 (* _returnvalue_10 _tilesize_2))
  (bind _returnvalue_12 (+ _returnvalue_11 _returnvalue_5))
  (bind _tile (CallFunction|GetTileXY (.x _returnvalue_4) (.y _returnvalue_4)))
  (return _tile (Math|Vector|MakeVector (.x _returnvalue_12) (.y _returnvalue_12) 0.0)))

(fn GetTileXY
  (params (x :type Integer) (y :type Integer))
  (return (Utilities|Array|Get(acopy) (Variables|Default|GetTileLayout) (+ x (* y (Variables|Default|GetTilesInChunk))))))

(fn IsCompatible
  (params (Chunk :type BP%20Chunk%20Parent%20Object%20Reference))
  (bind _returnvalue (Utilities|Enum|LiteralenumTileType "NewEnumerator0"))
  (for _index (range 0 (- (Variables|Default|GetTilesInChunk) 1))
    (if (and (Utilities|Enum|Equal(Enum) (Utilities|Array|Get(acopy) (Variables|BP_Chunk_Parent_C|GetTileLayout Chunk) _index) _returnvalue) (Utilities|Enum|Equal(Enum) (Utilities|Array|Get(acopy) (Variables|Default|GetTileLayout) (+ _index (- (* (Variables|Default|GetTilesInChunk) (Variables|Default|GetTilesInChunk)) (Variables|Default|GetTilesInChunk)))) _returnvalue))
      (return true)))
  (return false))