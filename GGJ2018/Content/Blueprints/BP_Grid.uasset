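; BP_Grid builds the game's tile grid from a list of chunk classes and answers position lookups on it.
; BeginPlay spawns the chunks edge to edge in a single row along Y, sized from tile size and tiles per chunk.
; GetChunk indexes that row by Y position, and GetTile passes the chunk-relative position to that chunk's own GetTile.
; SnapToTile returns the tile center at zero height.
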(event EventBeginPlay
  (bind _chunklist (Variables|Default|GetChunkList))
  (bind _chunksize (Variables|Default|GetChunkSize))
  (for _index (range 0 (Utilities|Array|Length _chunklist))
    (bind _returnvalue (Game|SpawnActorfromClass (Utilities|Array|Get(acopy) _chunklist _index) (Math|Conversions|ToTransform(Vector) (Math|Vector|MakeVector (* _chunksize 0.5) (* (+ (Math|Conversions|ToFloat(Integer) _index) 0.5) _chunksize) 0.0)) "Undefined" 0 0))
    (Utilities|Array|SetArrayElem (Variables|Default|GetChunks) _index _returnvalue)))

(event Collision|EventActorBeginOverlap
  (params (OtherActor :type Actor%20Object%20Reference)))

(event EventTick
  (params (DeltaSeconds :type Float%20%28single-precision%29)))

(fn ConstructionScript
  (Utilities|Array|Resize (Variables|Default|GetChunks) (Utilities|Array|Length (Variables|Default|GetChunkList)))
  (Variables|Default|SetChunkSize (* (Variables|Default|GetTileSize) (Math|Conversions|ToFloat(Integer) (Variables|Default|GetTilesInChunk)))))

(fn GetChunk
  (params (Position :type Vector))
  (return (Utilities|Array|Get(acopy) (Variables|Default|GetChunks) (Math|Float|Truncate (/ (.y Position) (Variables|Default|GetChunkSize))))))

(fn GetTile
  (params (Position :type Vector))
  (bind _chunksize (Variables|Default|GetChunkSize))
  (bind _returnvalue (* _chunksize 0.5))
  (bind _chunk (CallFunction|GetChunk Position))
  (bind (_tile _tilecenter) (Default|GetTile _chunk (- Position (- (Transformation|GetWorldLocation (Variables|/Game/Blueprints/BP_Chunk_Parent.BP_Chunk_Parent_C|GetDefaultSceneRoot _chunk)) (Math|Vector|MakeVector _returnvalue _returnvalue 0.0)))))
  (return _tile _tilecenter))

(fn SnaptoTile
  (params (Position :type Vector))
  (bind _tilesize (Variables|Default|GetTileSize))
  (bind _tilesize_2 (Variables|Default|GetTileSize))
  (bind _returnvalue (/ Position _tilesize))
  (bind _returnvalue_2 (Class|KismetMathLibrary|FTruncVector _returnvalue))
  (bind _returnvalue_3 (Math|Conversions|ToVector(Float) _returnvalue_2))
  (bind _returnvalue_4 (+ _returnvalue_3 0.5))
  (bind _returnvalue_5 (* _returnvalue_4 _tilesize_2))
  (return (Math|Vector|MakeVector (.x _returnvalue_5) (.y _returnvalue_5) 0.0)))