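; Placeable tower actor that follows the cursor, snapped to the game mode's grid, once the game has started and until it is placed.
; PlaceTower locks it and spawns four orthogonally adjacent Bp_TestTile actors, plus an outer diamond of eight if Upgraded.
; Each tile receives the tower's Action and a back-reference as owner.
; Tick also destroys the tower, behind a two-second Delay, when it projects past the screen's left edge.
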(event Custom|UpgradeTower
  (bind _returnvalue (Transformation|GetActorLocation))
  (bind _returnvalue_2 (Transformation|GetActorLocation))
  (bind _returnvalue_3 (Transformation|GetActorLocation))
  (bind _returnvalue_4 (Transformation|GetActorLocation))
  (bind _returnvalue_5 (Transformation|GetActorLocation))
  (bind _returnvalue_6 (Transformation|GetActorLocation))
  (bind _returnvalue_7 (Transformation|GetActorLocation))
  (bind _returnvalue_8 (Transformation|GetActorLocation))
  (bind _tileoffset (Variables|Default|GetTileOffset))
  (bind _tileoffset_2 (Variables|Default|GetTileOffset))
  (bind _tileoffset_3 (Variables|Default|GetTileOffset))
  (bind _tileoffset_4 (Variables|Default|GetTileOffset))
  (Utilities|FlowControl|Sequence
    (:then_0
      (bind _returnvalue_9 (Game|SpawnActorfromClass "/Game/Blueprints/Testing/bp_TestTile.bp_TestTile_C" (Math|Transform|MakeTransform (Math|Vector|MakeVector (.x _returnvalue_2) (+ (.y _returnvalue_2) (* (Variables|Default|GetTileOffset) 2.0)) (.z _returnvalue_2)) "0, 0, 0" "1,1,1") "AlwaysSpawn" 0 0))
      (Variables|/Game/Blueprints/Testing/bp_TestTile.bp_TestTile_C|SetAction _returnvalue_9 (Variables|Default|GetAction))
      (Variables|/Game/Blueprints/Testing/bp_TestTile.bp_TestTile_C|SetOwning%20Tower _returnvalue_9 self)
      (bind _returnvalue_10 (Game|SpawnActorfromClass "/Game/Blueprints/Testing/bp_TestTile.bp_TestTile_C" (Math|Transform|MakeTransform (Math|Vector|MakeVector (.x _returnvalue_3) (- (.y _returnvalue_3) (* (Variables|Default|GetTileOffset) 2.0)) (.z _returnvalue_3)) "0, 0, 0" "1,1,1") "AlwaysSpawn" 0 0))
      (Variables|/Game/Blueprints/Testing/bp_TestTile.bp_TestTile_C|SetAction _returnvalue_10 (Variables|Default|GetAction))
      (Variables|/Game/Blueprints/Testing/bp_TestTile.bp_TestTile_C|SetOwning%20Tower _returnvalue_10 self))
    (:then_1
      (bind _returnvalue_11 (Game|SpawnActorfromClass "/Game/Blueprints/Testing/bp_TestTile.bp_TestTile_C" (Math|Transform|MakeTransform (Math|Vector|MakeVector (+ (.x _returnvalue_5) (* (Variables|Default|GetTileOffset) 2.0)) (.y _returnvalue_5) (.z _returnvalue_5)) "0, 0, 0" "1,1,1") "AlwaysSpawn" 0 0))
      (Variables|/Game/Blueprints/Testing/bp_TestTile.bp_TestTile_C|SetAction _returnvalue_11 (Variables|Default|GetAction))
      (Variables|/Game/Blueprints/Testing/bp_TestTile.bp_TestTile_C|SetOwning%20Tower _returnvalue_11 self)
      (bind _returnvalue_12 (Game|SpawnActorfromClass "/Game/Blueprints/Testing/bp_TestTile.bp_TestTile_C" (Math|Transform|MakeTransform (Math|Vector|MakeVector (- (.x _returnvalue_6) (* (Variables|Default|GetTileOffset) 2.0)) (.y _returnvalue_6) (.z _returnvalue_6)) "0, 0, 0" "1,1,1") "AlwaysSpawn" 0 0))
      (Variables|/Game/Blueprints/Testing/bp_TestTile.bp_TestTile_C|SetAction _returnvalue_12 (Variables|Default|GetAction))
      (Variables|/Game/Blueprints/Testing/bp_TestTile.bp_TestTile_C|SetOwning%20Tower _returnvalue_12 self))
    (:then_2
      (bind _returnvalue_13 (Game|SpawnActorfromClass "/Game/Blueprints/Testing/bp_TestTile.bp_TestTile_C" (Math|Transform|MakeTransform (Math|Vector|MakeVector (+ (.x _returnvalue_7) _tileoffset_2) (+ (.y _returnvalue_7) _tileoffset_2) (.z _returnvalue_7)) "0, 0, 0" "1,1,1") "AlwaysSpawn" 0 0))
      (Variables|/Game/Blueprints/Testing/bp_TestTile.bp_TestTile_C|SetAction _returnvalue_13 (Variables|Default|GetAction))
      (Variables|/Game/Blueprints/Testing/bp_TestTile.bp_TestTile_C|SetOwning%20Tower _returnvalue_13 self)
      (bind _returnvalue_14 (Game|SpawnActorfromClass "/Game/Blueprints/Testing/bp_TestTile.bp_TestTile_C" (Math|Transform|MakeTransform (Math|Vector|MakeVector (- (.x _returnvalue_8) _tileoffset_3) (- (.y _returnvalue_8) _tileoffset_3) (.z _returnvalue_8)) "0, 0, 0" "1,1,1") "AlwaysSpawn" 0 0))
      (Variables|/Game/Blueprints/Testing/bp_TestTile.bp_TestTile_C|SetAction _returnvalue_14 (Variables|Default|GetAction))
      (Variables|/Game/Blueprints/Testing/bp_TestTile.bp_TestTile_C|SetOwning%20Tower _returnvalue_14 self))
    (:then_3
      (bind _returnvalue_15 (Game|SpawnActorfromClass "/Game/Blueprints/Testing/bp_TestTile.bp_TestTile_C" (Math|Transform|MakeTransform (Math|Vector|MakeVector (- (.x _returnvalue) _tileoffset) (+ (.y _returnvalue) _tileoffset) (.z _returnvalue)) "0, 0, 0" "1,1,1") "AlwaysSpawn" 0 0))
      (Variables|/Game/Blueprints/Testing/bp_TestTile.bp_TestTile_C|SetAction _returnvalue_15 (Variables|Default|GetAction))
      (Variables|/Game/Blueprints/Testing/bp_TestTile.bp_TestTile_C|SetOwning%20Tower _returnvalue_15 self)
      (bind _returnvalue_16 (Game|SpawnActorfromClass "/Game/Blueprints/Testing/bp_TestTile.bp_TestTile_C" (Math|Transform|MakeTransform (Math|Vector|MakeVector (+ (.x _returnvalue_4) _tileoffset_4) (- (.y _returnvalue_4) _tileoffset_4) (.z _returnvalue_4)) "0, 0, 0" "1,1,1") "AlwaysSpawn" 0 0))
      (Variables|/Game/Blueprints/Testing/bp_TestTile.bp_TestTile_C|SetAction _returnvalue_16 (Variables|Default|GetAction))
      (Variables|/Game/Blueprints/Testing/bp_TestTile.bp_TestTile_C|SetOwning%20Tower _returnvalue_16 self))))

(event Custom|PlaceTower
  (Variables|Default|SetIsPlaced true)
  (CallFunction|SetTower)
  (if (Variables|Default|GetUpgraded)
    (CallFunction|UpgradeTower)))

(event Custom|SetTower
  (bind _returnvalue (Transformation|GetActorLocation))
  (bind _returnvalue_2 (Transformation|GetActorLocation))
  (bind _returnvalue_3 (Transformation|GetActorLocation))
  (bind _returnvalue_4 (Transformation|GetActorLocation))
  (Utilities|FlowControl|Sequence
    (:then_0
      (bind _returnvalue_5 (Game|SpawnActorfromClass "/Game/Blueprints/Testing/bp_TestTile.bp_TestTile_C" (Math|Transform|MakeTransform (Math|Vector|MakeVector (.x _returnvalue) (+ (.y _returnvalue) (Variables|Default|GetTileOffset)) (.z _returnvalue)) "0, 0, 0" "1,1,1") "AlwaysSpawn" 0 0))
      (Variables|/Game/Blueprints/Testing/bp_TestTile.bp_TestTile_C|SetAction _returnvalue_5 (Variables|Default|GetAction))
      (Variables|/Game/Blueprints/Testing/bp_TestTile.bp_TestTile_C|SetOwning%20Tower _returnvalue_5 self)
      (bind _returnvalue_6 (Game|SpawnActorfromClass "/Game/Blueprints/Testing/bp_TestTile.bp_TestTile_C" (Math|Transform|MakeTransform (Math|Vector|MakeVector (.x _returnvalue_3) (- (.y _returnvalue_3) (Variables|Default|GetTileOffset)) (.z _returnvalue_3)) "0, 0, 0" "1,1,1") "AlwaysSpawn" 0 0))
      (Variables|/Game/Blueprints/Testing/bp_TestTile.bp_TestTile_C|SetAction _returnvalue_6 (Variables|Default|GetAction))
      (Variables|/Game/Blueprints/Testing/bp_TestTile.bp_TestTile_C|SetOwning%20Tower _returnvalue_6 self))
    (:then_1
      (bind _returnvalue_7 (Game|SpawnActorfromClass "/Game/Blueprints/Testing/bp_TestTile.bp_TestTile_C" (Math|Transform|MakeTransform (Math|Vector|MakeVector (+ (.x _returnvalue_2) (Variables|Default|GetTileOffset)) (.y _returnvalue_2) (.z _returnvalue_2)) "0, 0, 0" "1,1,1") "AlwaysSpawn" 0 0))
      (Variables|/Game/Blueprints/Testing/bp_TestTile.bp_TestTile_C|SetAction _returnvalue_7 (Variables|Default|GetAction))
      (Variables|/Game/Blueprints/Testing/bp_TestTile.bp_TestTile_C|SetOwning%20Tower _returnvalue_7 self)
      (bind _returnvalue_8 (Game|SpawnActorfromClass "/Game/Blueprints/Testing/bp_TestTile.bp_TestTile_C" (Math|Transform|MakeTransform (Math|Vector|MakeVector (- (.x _returnvalue_4) (Variables|Default|GetTileOffset)) (.y _returnvalue_4) (.z _returnvalue_4)) "0, 0, 0" "1,1,1") "AlwaysSpawn" 0 0))
      (Variables|/Game/Blueprints/Testing/bp_TestTile.bp_TestTile_C|SetAction _returnvalue_8 (Variables|Default|GetAction))
      (Variables|/Game/Blueprints/Testing/bp_TestTile.bp_TestTile_C|SetOwning%20Tower _returnvalue_8 self))))

(event EventTick
  (params (DeltaSeconds :type Float%20%28single-precision%29))
  (bind _returnvalue (Game|GetPlayerController 0))
  (bind _array (Utilities|Array|MakeArray "ObjectTypeQuery1"))
  (bind _hitresult (Class|PlayerController|GetHitResultUnderCursorforObjects _returnvalue _array false))
  (Utilities|FlowControl|Sequence
    (:then_0
      (Utilities|FlowControl|Delay 2.0)
      (if (<= (.x (.ScreenPosition (Class|GameplayStatics|ProjectWorldtoScreen (Game|GetPlayerController 0) (Transformation|GetWorldLocation (Variables|Default|GetTower)) false))) -5e+01)
        (Actor|DestroyActor)))
    (:then_1
      (bind _asbp_game_mode (Utilities|Casting|CastTobp_GameMode (Game|GetGameMode)))
      (if (Variables|/Game/Blueprints/bp_GameMode.bp_GameMode_C|GetStarted _asbp_game_mode)
        (if (not (Variables|Default|GetIsPlaced))
          (bind _asbp_game_mode_2 (Utilities|Casting|CastTobp_GameMode (Game|GetGameMode)))
          (bind _snappedposition (Default|SnaptoTile (Variables|/Game/Blueprints/bp_GameMode.bp_GameMode_C|Getgrid _asbp_game_mode_2) (Math|Vector|MakeVector (.x (.location _hitresult)) (.y (.location _hitresult)) (.z (.location _hitresult)))))
          (Transformation|SetActorLocation (Math|Vector|MakeVector (.x _snappedposition) (.y _snappedposition) (.z (.location _hitresult))) false true))))))

(fn ConstructionScript)