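; A debug dummy actor that follows the mouse cursor until it is placed in the world.
; Each tick while unplaced, it teleports to the player controller's under-cursor hit location against WorldStatic objects.
; Releasing the left mouse button sets IsPlaced, which freezes it in position; the construction script resets the flag to false.
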(event EventBeginPlay)

(event Collision|EventActorBeginOverlap
  (params (OtherActor :type Actor%20Object%20Reference)))

(event EventTick
  (params (DeltaSeconds :type Float%20%28single-precision%29))
  (if (not (Variables|Default|GetIsPlaced))
    (Transformation|SetActorLocation (.location (.HitResult (Class|PlayerController|GetHitResultUnderCursorforObjects (Game|GetPlayerController 0) (Utilities|Array|MakeArray "ObjectTypeQuery1") false))) false true)))

(event Input|MouseEvents|LeftMouseButton
  (params (Key :type Key%20Structure))
  (:Released
    (if (not (Variables|Default|GetIsPlaced))
      (Variables|Default|SetIsPlaced true))))

(fn ConstructionScript
  (Variables|Default|SetIsPlaced false))